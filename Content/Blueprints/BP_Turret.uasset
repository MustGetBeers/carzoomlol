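; BP_Turret is a turret that tracks and fires at the player, started and stopped by trigger events from the BPI_turret interface.
; Entering the trigger opens a Gate that snaps the actor to face player pawn 0, then spawns a BP_Projectile at BulletSpawner after a short delay.
; Each shot re-enters the Gate to form a repeating aim-and-fire loop, which ends when the exit event closes it.
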(event EventEnterTurretTrigger
  (params (Is%20in%20trigger? :type Boolean))
  ;[1 1 1] triggered via BPI_turret interface and BP_trigger_sense triggers
  (Utilities|FlowControl|Sequence
    (:then_0
      (goto _label Open))
    (:then_1
      (Utilities|FlowControl|Gate false :!label _label
        (:Exit
          ;[1 1 1] finds player, sets the turret to look at the location of the player
          (Utilities|FlowControl|Sequence
            (:then_0
              (Transformation|SetActorRotation (Math|Rotator|FindLookatRotation (Transformation|GetActorLocation) (Transformation|GetActorLocation (Game|Player|GetPlayerPawn 0)))))
            (:then_1
              ;[1 1 1] Fires the projectile at the player
              (Utilities|FlowControl|Delay 0.3)
              (Game|SpawnActorfromClass "/Game/Blueprints/BP_Projectile.BP_Projectile_C" (Transformation|GetWorldTransform (Variables|Default|GetbulletSpawner)) "Undefined" 0 0)
              (goto _label))))))))

(event EventExitTurretTrigger
  ;[1 1 1] triggered via BPI_turret interface and BP_trigger_sense triggers
  (Utilities|FlowControl|Gate false) ; enters at Close
)

(fn ConstructionScript)