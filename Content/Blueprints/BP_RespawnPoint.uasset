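; Respawn point for the vehicle game, acting as a checkpoint that records where the player's car respawns.
; When a PP_SampleVehicleUseThis overlaps SpawnDetector, the vehicle's own transform, not the point's, is saved as SpawnTransform on the CarZOom game mode.
; On BeginPlay it also makes player controller 0 possess the first actor found of the game mode's default pawn class.
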(event OnComponentBeginOverlap(SpawnDetector)
  (params (OverlappedComponent :type Primitive%20Component%20Object%20Reference) (OtherActor :type Actor%20Object%20Reference) (OtherComp :type Primitive%20Component%20Object%20Reference) (OtherBodyIndex :type Integer) (bFromSweep :type Boolean) (SweepResult :type Hit%20Result%20Structure%20%28by%20ref%29))
  (bind _aspp_sample_vehicle_use_this (Utilities|Casting|CastToPP_SampleVehicleUseThis OtherActor))
  (bind _ascar_zoom (Utilities|Casting|CastToCarZOom (Game|GetGameMode)))
  (Variables|/Game/Blueprints/CarZOom.CarZOom_C|SetSpawnTransform _ascar_zoom (Transformation|GetActorTransform _aspp_sample_vehicle_use_this)))

(event EventBeginPlay
  (bind _returnvalue (Game|GetGameMode))
  (Class|GameModeBase|GetDefaultPawnClassforController _returnvalue)
  (bind _returnvalue_2 (Actor|GetActorOfClass (Variables|/Script/Engine.GameModeBase|GetDefaultPawnClass _returnvalue)))
  (Pawn|Possess (Game|GetPlayerController 0) _returnvalue_2))

(fn ConstructionScript)