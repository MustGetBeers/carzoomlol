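; CarZOom runs the game flow for a timed vehicle game, from start screen to game over.
; BeginPlay shows the start widget, pauses, and binds to the player vehicle's destruction, which triggers a delayed spawn, possession and rebind.
; A Tick-driven one-second Delay counts down minutes and seconds, then shows game over, calls the GameInstance's coin message reset and pauses.
; GetCoin only returns zero.
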(event Custom|OnDestroyed_
  (params (DestroyedActor :type Actor%20Object%20Reference))
  ;[1 0 0.9141] Change this from binding to interface
  (Utilities|FlowControl|Delay (Variables|Default|GetSpawnDelay))
  (bind _returnvalue (Game|SpawnActorfromClass "/Game/Blueprints/PP_SampleVehicleUseThis.PP_SampleVehicleUseThis_C" (Variables|Default|GetSpawnTransform) "Undefined" 0 0))
  (Pawn|Possess (Game|GetPlayerController 0) _returnvalue)
  (CallFunction|Respawn))

(event Custom|Respawn
  ;[1 0 0.9141] Change this from binding to interface
  (bind _aspp_sample_vehicle_use_this (Utilities|Casting|CastToPP_SampleVehicleUseThis (Game|Player|GetPlayerPawn 0)))
  (Game|BindEventtoOnDestroyed _aspp_sample_vehicle_use_this (delegate Custom|OnDestroyed_)))

(event EventBeginPlay
  (bind _returnvalue (UserInterface|CreateWidget "/Game/Blueprints/UI_StartGame.UI_StartGame_C"))
  (UserInterface|Viewport|AddtoViewport _returnvalue 0)
  (Variables|/Script/Engine.PlayerController|SetbShowMouseCursor (Game|GetPlayerController 0) true)
  (Game|SetGamePaused true)
  ;[1 0 0.9141] Change this from binding to interface
  (bind _aspp_sample_vehicle_use_this (Utilities|Casting|CastToPP_SampleVehicleUseThis (Game|Player|GetPlayerPawn 0)))
  (Game|BindEventtoOnDestroyed _aspp_sample_vehicle_use_this (delegate Custom|OnDestroyed_)))

(event EventTick
  (params (DeltaSeconds :type Float%20%28single-precision%29))
  (Utilities|FlowControl|Delay 1.0)
  ;[0.1953 1 0] weird countdown nodes, which eventually reach 0 for minutes and seconds in which case it ceates the game over widget
  (if (== (Variables|Default|GetSeconds) 0)
    (if (== (Variables|Default|GetMinutes) 0)
      (bind _returnvalue (UserInterface|CreateWidget "/Game/Blueprints/UI_GameOver.UI_GameOver_C"))
      (UserInterface|Viewport|AddtoViewport _returnvalue 0)
      (Variables|/Script/Engine.PlayerController|SetbShowMouseCursor (Game|GetPlayerController 0) true)
      (Class|BPICoinCounter|ResetCoin(Message) (Game|GetGameInstance) (Variables|Default|GetN))
      (Game|SetGamePaused true)
      (else
        (Variables|Default|SetSeconds 59)
        (Variables|Default|SetMinutes (- (Variables|Default|GetMinutes) 1))))
    (else
      (Variables|Default|SetSeconds (- (Variables|Default|GetSeconds) 1)))))

(fn ConstructionScript)

(fn GetCoin
  (return 0))