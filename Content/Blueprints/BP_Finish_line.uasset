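; Finish line actor that loads the level map_2 when the player pawn overlaps its FinishBox.
; On BeginPlay it passes itself and its Disabled flag to DisableActor, then after a short delay clears the flag and calls DisableActor again.
; The overlap handler checks only for the first player's pawn and prints a message before opening the level.
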(event OnComponentBeginOverlap(finishbox)
  (params (OverlappedComponent :type Primitive%20Component%20Object%20Reference) (OtherActor :type Actor%20Object%20Reference) (OtherComp :type Primitive%20Component%20Object%20Reference) (OtherBodyIndex :type Integer) (bFromSweep :type Boolean) (SweepResult :type Hit%20Result%20Structure%20%28by%20ref%29))
  (if (== (Game|Player|GetPlayerPawn 0) OtherActor)
    (Development|PrintString "passed")
    (Game|OpenLevel(byName) "map_2")))

(event EventBeginPlay
  (bind _self self)
  (CallFunction|DisableActor (Variables|Default|GetDisabled) _self)
  (Utilities|FlowControl|Delay 5.0)
  (bind _output_get (Variables|Default|SetDisabled false))
  (CallFunction|DisableActor _output_get _self))

(fn ConstructionScript)